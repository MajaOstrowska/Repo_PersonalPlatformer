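; Player controller Blueprint that puts up the HUD and toggles the in-game inventory menu.
; BeginPlay creates the HUD_Canvas widget and adds it to the viewport.
; The I key creates a fresh IngameMenu or removes the open one, flipping the BlockControls flag, mouse cursor and input mode between Game-and-UI and Game-Only.
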(event `Key|I`
  (params (Key :type "Key Structure"))
  (bind _returnvalue (`GameplayStatics.GetPlayerController` 0))
  ;[1 1 1] ingame inventory on pressed i
  (:`Pressed`
    (if (`self.IsMenuClosed`)
      (set `self.BlockControls` true)
      (bind _returnvalue_2 (`|CreateWidget` "/Game/Menu/IngameMenu.IngameMenu_C" _returnvalue))
      (bind _output_get (set `self.Menu` _returnvalue_2))
      (`UserWidget.AddToViewport` _output_get 1)
      (set `PlayerController.bShowMouseCursor` true _returnvalue)
      (set `self.IsMenuClosed` false)
      (`WidgetBlueprintLibrary.SetInputMode_GameAndUIEx` (`GameplayStatics.GetPlayerController` 0) (`self.Menu`) "DoNotLock" false)
      (else
        (set `self.BlockControls` false)
        (`Widget.RemoveFromParent` (`self.Menu`))
        (set `PlayerController.bShowMouseCursor` false (`GameplayStatics.GetPlayerController` 0))
        (set `self.IsMenuClosed` true)
        (`WidgetBlueprintLibrary.SetInputMode_GameOnly` (`GameplayStatics.GetPlayerController` 0))))))

(event `self.ReceiveBeginPlay`
  (bind _returnvalue (`|CreateWidget` "/Game/InventorySystem/HUD_Canvas.HUD_Canvas_C"))
  (bind _output_get (set `self.HUD` _returnvalue))
  (`UserWidget.AddToViewport` _output_get 0))

(fn `UserConstructionScript`)